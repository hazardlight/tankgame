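; Mortar_BP is a mortar actor that aims through a TankAiming component driving its barrel and turret.
; On BeginPlay it assigns Projectile_BP as the projectile and initializes the aiming component with the Barrel and Turret.
; It then links its widget component's HealthBar to itself as the Tank to display.
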(event `self.ReceiveBeginPlay`
  (set `TankAimingComponent.ProjectileBlueprint` "/Game/Tank/Projectile_BP.Projectile_BP_C" (`self.TankAiming`))
  (`TankAimingComponent.Initialize` (`self.TankAiming`) (`self.Barrel`) (`self.Turret`))
  (bind _ashealth_bar (cast `/Game/UI/HealthBar` (`WidgetComponent.GetUserWidgetObject` (`self.Widget`))))
  (set `/Game/UI/HealthBar.Tank` self _ashealth_bar))

(fn `UserConstructionScript`)