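; Tank pawn Blueprint that wires player input to driving, camera aiming and firing.
; BeginPlay hands the barrel and turret to TankAiming, and both tracks to TankMovement.
; Aim axes rotate an azimuth gimbal and spring arm, scaled by frame time, while Fire calls the fire function.
; Driving has two paths: throttle axes set each track directly, while move and turn axes send intents to TankMovement.
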(event `self.ReceiveBeginPlay`
  (`TankAimingComponent.Initialize` (`self.TankAiming`) (`self.Barrel`) (`self.Turret`))
  (`TankMovementComponent.Initialize` (`self.TankMovement`) (`self.Left Track`) (`self.Right Track`)))

(event `InputAxis|AimAzimuth`
  (params (AxisValue :type "Float (single-precision)"))
  ;[1 1 1] Camera Input Binding
  (`SceneComponent.K2_AddLocalRotation` (`self.Azimuth Gimbal`) (`KismetMathLibrary.MakeRotator` 0.0 0.0 (* AxisValue (`GameplayStatics.GetWorldDeltaSeconds`) 100.0)) false false))

(event `InputAxis|AimElevation`
  (params (AxisValue :type "Float (single-precision)"))
  ;[1 1 1] Camera Input Binding
  (`SceneComponent.K2_AddLocalRotation` (`self.SpringArm`) (`KismetMathLibrary.MakeRotator` 0.0 (* AxisValue (`GameplayStatics.GetWorldDeltaSeconds`) 100.0)) false false))

(event `InputAxis|Throttle Forward`
  (params (AxisValue :type "Float (single-precision)"))
  (`TankTrack.SetThrottle` (`self.Left Track`) AxisValue)
  (`TankTrack.SetThrottle` (`self.Right Track`) AxisValue))

(event `InputAxis|Throttle Right`
  (params (AxisValue :type "Float (single-precision)"))
  (`TankTrack.SetThrottle` (`self.Left Track`) AxisValue)
  (bind _result (`/Engine/EditorBlueprintResources/StandardMacros.NegateFloat` AxisValue)
    (:`  `
      (`TankTrack.SetThrottle` (`self.Right Track`) (/ _result 2.0)))))

(event `InputAxis|Throttle Left`
  (params (AxisValue :type "Float (single-precision)"))
  (`TankTrack.SetThrottle` (`self.Right Track`) AxisValue)
  (bind _result (`/Engine/EditorBlueprintResources/StandardMacros.NegateFloat` AxisValue)
    (:`  `
      (`TankTrack.SetThrottle` (`self.Left Track`) (/ _result 2.0)))))

(event `InputAction|Fire`
  (params (Key :type "Key Structure"))
  (:`Pressed`
    (`self.Fire`)))

(event `InputAxis|Move Forward`
  (params (AxisValue :type "Float (single-precision)"))
  (`TankMovementComponent.IntendMoveForward` (`self.TankMovement`) AxisValue))

(event `InputAxis|Turn Right`
  (params (AxisValue :type "Float (single-precision)"))
  (`TankMovementComponent.IntendTurnRight` (`self.TankMovement`) AxisValue))

(event `InputAxis|Turn Left`
  (params (AxisValue :type "Float (single-precision)"))
  (`TankMovementComponent.IntendTurnLeft` (`self.TankMovement`) AxisValue))

(fn `UserConstructionScript`)